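; BP_DeliveryPost is a delivery point that accepts packages matching its DeliveryID, which it shows as text at BeginPlay.
; Collider overlap by the third-person character swaps the marker for a prompt and enables interact input until a delivery is made.
; Interacting destroys matching packages and removes them from the player's inventory component, hides marker and prompt, then updates the character's quest and notifies BP_NextLevelPortal.
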(event OnComponentBeginOverlap(Collider)
  (params (OverlappedComponent :type Primitive%20Component%20Object%20Reference) (OtherActor :type Actor%20Object%20Reference) (OtherComp :type Primitive%20Component%20Object%20Reference) (OtherBodyIndex :type Integer) (bFromSweep :type Boolean) (SweepResult :type Hit%20Result%20Structure%20%28by%20ref%29))
  ;[1 1 1] Marker Visibility - CF
  (Utilities|Casting|CastToBP_ThirdPersonCharacter OtherActor)
  (if (not (Variables|Default|GetHasDeliveryBeenMade))
    (Rendering|SetVisibility (Variables|Default|GetMarker) false true)
    (Rendering|SetVisibility (Variables|Default|GetPrompt) true false)
    (Input|EnableInput (Game|GetPlayerController 0))))

(event OnComponentEndOverlap(Collider)
  (params (OverlappedComponent :type Primitive%20Component%20Object%20Reference) (OtherActor :type Actor%20Object%20Reference) (OtherComp :type Primitive%20Component%20Object%20Reference) (OtherBodyIndex :type Integer))
  ;[1 1 1] Marker Visibility - CF
  (Utilities|Casting|CastToBP_ThirdPersonCharacter OtherActor)
  (if (not (Variables|Default|GetHasDeliveryBeenMade))
    (Rendering|SetVisibility (Variables|Default|GetMarker) true true)
    (Rendering|SetVisibility (Variables|Default|GetPrompt) false false)
    (Input|DisableInput (Game|GetPlayerController 0))))

(event Input|EnhancedActionEvents|EnhancedInputActionIA_Interact
  (params (ActionValue :type Boolean) (ElapsedSeconds :type Float%20%28double-precision%29) (TriggeredSeconds :type Float%20%28double-precision%29) (InputAction :type Input%20Action%20Object%20Reference :default "/Game/Dynamic/ThirdPerson/Input/Actions/IA_Interact.IA_Interact"))
  ;[1 1 1] Deliver Package Check - CF
  (:Triggered
    (bind _asbp_third_person_character (Utilities|Casting|CastToBP_ThirdPersonCharacter (Game|GetPlayerCharacter 0)))
    (for _array_element (Variables|/Game/Dynamic/ThirdPerson/Blueprints/BPC_Inventory.BPC_Inventory_C|GetPackages (Variables|/Game/Dynamic/ThirdPerson/Blueprints/BP_ThirdPersonCharacter.BP_ThirdPersonCharacter_C|GetBPC_Inventory _asbp_third_person_character))
      (if (== (Variables|/Game/Dynamic/Blueprints/BP_Package.BP_Package_C|GetDeliveryID _array_element) (Variables|Default|GetDeliveryID))
        (Actor|DestroyActor _array_element)
        (Default|RemoveItemfromPackages (Variables|/Game/Dynamic/ThirdPerson/Blueprints/BP_ThirdPersonCharacter.BP_ThirdPersonCharacter_C|GetBPC_Inventory _asbp_third_person_character) _array_element)
        (Variables|Default|SetHasDeliveryBeenMade true)
        (Rendering|SetVisibility (Variables|Default|GetMarker) false false)
        (Rendering|SetVisibility (Variables|Default|GetPrompt) false false)
        ;[1 1 1] Update quest objective - CF
        (bind _returnvalue (Actor|GetActorOfClass "/Game/Dynamic/ThirdPerson/Blueprints/BP_ThirdPersonCharacter.BP_ThirdPersonCharacter_C"))
        (Default|UpdateQuest _returnvalue)
        ;[1 1 1] Updates next level door prompt - CF
        (bind _returnvalue_2 (Actor|GetActorOfClass "/Game/Dynamic/Blueprints/BP_NextLevelPortal.BP_NextLevelPortal_C"))
        (Default|ObjectivesComplete _returnvalue_2)))))

(event EventBeginPlay
  ;[1 1 1] Updates ID in gameworld - CF
  (Rendering|Components|TextRender|SetText (Variables|Default|GetIDNumber) (Utilities|Text|ToText(Integer) (Variables|Default|GetDeliveryID))))

(fn ConstructionScript)