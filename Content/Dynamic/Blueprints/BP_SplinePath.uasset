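; Spline path actor for flying sequences that drives the player's third-person camera along its spline.
; The enter collider registers the path on the character, triggers flying and camera state, and starts a delay-based loop that advances the camera while flying.
; One path type rotates and offsets the camera for a reversed view.
; The exit collider, moved to the spline's end on BeginPlay, switches flying state; RejoinSpline resumes the loop.
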(event OnComponentBeginOverlap(EnterCollider)
  (params (OverlappedComponent :type Primitive%20Component%20Object%20Reference) (OtherActor :type Actor%20Object%20Reference) (OtherComp :type Primitive%20Component%20Object%20Reference) (OtherBodyIndex :type Integer) (bFromSweep :type Boolean) (SweepResult :type Hit%20Result%20Structure%20%28by%20ref%29))
  ;[1 1 1] Starts flying sequence - CF
  (bind _asbp_third_person_character (Utilities|Casting|CastToBP_ThirdPersonCharacter OtherActor))
  (Variables|Default|SetPlayerCharacter _asbp_third_person_character)
  (Variables|/Game/Dynamic/ThirdPerson/Blueprints/BP_ThirdPersonCharacter.BP_ThirdPersonCharacter_C|SetCurrentSpline _asbp_third_person_character self)
  (Default|TriggerFlying _asbp_third_person_character "NewEnumerator0")
  (Default|UpdateCameraState _asbp_third_person_character "NewEnumerator0")
  ;[1 1 1] Sets cameras rotation and location
  (if (Utilities|Enum|Equal(Enum) (Variables|Default|GetTypeOfPath) "NewEnumerator1")
    (Variables|Default|SetReverseRotator "180.000000,0.000000,180.000000")
    (Variables|Default|SetReverseLocation 6e+02)
    (else
      (Variables|Default|SetReverseRotator "0, 0, 0")
      (Variables|Default|SetReverseLocation 0.0)))
  ;[1 1 1] Trigger Spline Movement
  (if (< (Variables|Default|GetDistanceAlongSpline) (Spline|GetSplineLength (Variables|Default|GetSpline))) :!label _label
    (CallFunction|MoveAlongSpline)
    (Utilities|FlowControl|Delay (Class|Actor|GetActorTickInterval))
    (if (Utilities|IsValid _asbp_third_person_character)
      (if (Class|NavMovementComponent|IsFlying (Variables|/Script/Engine.Character|GetCharacterMovement _asbp_third_person_character))
        (goto _label))
      (else
        (Variables|Default|SetDistanceAlongSpline 0.0)))))

(event OnComponentBeginOverlap(ExitCollider)
  (params (OverlappedComponent :type Primitive%20Component%20Object%20Reference) (OtherActor :type Actor%20Object%20Reference) (OtherComp :type Primitive%20Component%20Object%20Reference) (OtherBodyIndex :type Integer) (bFromSweep :type Boolean) (SweepResult :type Hit%20Result%20Structure%20%28by%20ref%29))
  ;[1 1 1] Ends flying sequence - CF
  (bind _asbp_third_person_character (Utilities|Casting|CastToBP_ThirdPersonCharacter OtherActor))
  (Default|TriggerFlying _asbp_third_person_character "NewEnumerator1")
  (Default|UpdateCameraState _asbp_third_person_character "NewEnumerator1"))

(event OnComponentEndOverlap(ExitCollider)
  (params (OverlappedComponent :type Primitive%20Component%20Object%20Reference) (OtherActor :type Actor%20Object%20Reference) (OtherComp :type Primitive%20Component%20Object%20Reference) (OtherBodyIndex :type Integer))
  ;[1 1 1] Resets distance along spline once player leaves area
  (Variables|Default|SetDistanceAlongSpline 0.0)
  (Variables|/Game/Dynamic/ThirdPerson/Blueprints/BP_ThirdPersonCharacter.BP_ThirdPersonCharacter_C|SetPlayerToFlyingStart (stale OnComponentBeginOverlap(ExitCollider) _asbp_third_person_character) false))

(event Custom|RejoinSpline
  ;[1 1 1] Trigger Spline Movement
  (if (< (Variables|Default|GetDistanceAlongSpline) (Spline|GetSplineLength (Variables|Default|GetSpline))) :!label _label
    (CallFunction|MoveAlongSpline)
    (Utilities|FlowControl|Delay (Class|Actor|GetActorTickInterval))
    (if (Utilities|IsValid (stale OnComponentBeginOverlap(EnterCollider) _asbp_third_person_character))
      (if (Class|NavMovementComponent|IsFlying (Variables|/Script/Engine.Character|GetCharacterMovement (stale OnComponentBeginOverlap(EnterCollider) _asbp_third_person_character)))
        (goto _label))
      (else
        (Variables|Default|SetDistanceAlongSpline 0.0)))))

(event Custom|MoveAlongSpline
  (bind _playercharacter (Variables|Default|GetPlayerCharacter))
  ;[1 1 1] Moves target along spline path - CF
  (Variables|Default|SetDistanceAlongSpline (+ (* (Utilities|Time|GetWorldDeltaSeconds) (Variables|Default|GetSplineSpeed)) (Variables|Default|GetDistanceAlongSpline)))
  (if (Utilities|IsValid _playercharacter)
    (Transformation|SetWorldTransform (Variables|/Game/Dynamic/ThirdPerson/Blueprints/BP_ThirdPersonCharacter.BP_ThirdPersonCharacter_C|Get3rdPersonCamera _playercharacter) (Math|Transform|MakeTransform (.location (Spline|GetTransformatDistanceAlongSpline (Variables|Default|GetSpline) (+ (Variables|Default|GetDistanceAlongSpline) (Variables|Default|GetReverseLocation)) "World" false)) (Math|Conversions|RotationFromXVector (Math|Vector|RotateVector (Math|Rotator|GetRotationXVector (.rotation (Spline|GetTransformatDistanceAlongSpline (Variables|Default|GetSpline) (+ (Variables|Default|GetDistanceAlongSpline) (Variables|Default|GetReverseLocation)) "World" false))) (Variables|Default|GetReverseRotator))) (Variables|/Script/Engine.SceneComponent|GetRelativeScale3D (Variables|/Game/Dynamic/ThirdPerson/Blueprints/BP_ThirdPersonCharacter.BP_ThirdPersonCharacter_C|Get3rdPersonCamera (Variables|Default|GetPlayerCharacter)))) false false)
    (else
      (Variables|Default|SetDistanceAlongSpline 0.0))))

(event EventBeginPlay
  (bind _spline (Variables|Default|GetSpline))
  ;[1 1 1] Sets exit collider position to end of spline - CF
  (Transformation|SetWorldLocation (Variables|Default|GetExitCollider) (Spline|GetLocationatDistanceAlongSpline _spline (Spline|GetSplineLength _spline) "World") false false))

(fn ConstructionScript)