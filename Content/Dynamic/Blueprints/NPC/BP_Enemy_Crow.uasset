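; Crow enemy NPC that damages the third-person player character on contact with its capsule.
; An overlap takes one point of player Health when CanDamage is set, then raises a HitImmunity flag that clears after a short delay once the player leaves the capsule.
; When Health reaches zero, it destroys both the player and itself.
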(event OnComponentBeginOverlap(CapsuleComponent)
  (params (OverlappedComponent :type Primitive%20Component%20Object%20Reference) (OtherActor :type Actor%20Object%20Reference) (OtherComp :type Primitive%20Component%20Object%20Reference) (OtherBodyIndex :type Integer) (bFromSweep :type Boolean) (SweepResult :type Hit%20Result%20Structure%20%28by%20ref%29))
  ;[1 1 1] Damage player - CF
  (if (not (Variables|Default|GetHitImmunity))
    (bind _asbp_third_person_character (Utilities|Casting|CastToBP_ThirdPersonCharacter OtherActor))
    (if (Variables|Default|GetCanDamage?)
      (CallFunction|DamagePlayer)
      (Variables|Default|SetHitImmunity true))))

(event OnComponentEndOverlap(CapsuleComponent)
  (params (OverlappedComponent :type Primitive%20Component%20Object%20Reference) (OtherActor :type Actor%20Object%20Reference) (OtherComp :type Primitive%20Component%20Object%20Reference) (OtherBodyIndex :type Integer))
  ;[1 1 1] DebugMode - CF
  (Utilities|Casting|CastToBP_ThirdPersonCharacter OtherActor)
  (Utilities|FlowControl|Delay 1.0)
  (Variables|Default|SetHitImmunity false))

(event Custom|DamagePlayer
  ;[1 1 1] Damage player - CF
  (bind _result (Math|Integer|DecrementInt (Variables|/Game/Dynamic/ThirdPerson/Blueprints/BP_ThirdPersonCharacter.BP_ThirdPersonCharacter_C|GetHealth (stale OnComponentBeginOverlap(CapsuleComponent) _asbp_third_person_character)))
    (:%20%20
      (Variables|/Game/Dynamic/ThirdPerson/Blueprints/BP_ThirdPersonCharacter.BP_ThirdPersonCharacter_C|SetHealth (stale OnComponentBeginOverlap(CapsuleComponent) _asbp_third_person_character) _result)
      (if (<= (Variables|/Game/Dynamic/ThirdPerson/Blueprints/BP_ThirdPersonCharacter.BP_ThirdPersonCharacter_C|GetHealth (stale OnComponentBeginOverlap(CapsuleComponent) _asbp_third_person_character)) 0)
        (Actor|DestroyActor (stale OnComponentBeginOverlap(CapsuleComponent) _asbp_third_person_character))
        (Actor|DestroyActor)))))

(fn ConstructionScript)