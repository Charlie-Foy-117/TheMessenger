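; BP_NPC is a talkable NPC with a flipbook sprite and line-by-line dialogue.
; Overlapping its collider shows the third-person character's interact prompt, and leaving hides prompt and dialogue and resets the line index.
; Talk steps through the Dialogue array in a lazily created, reused WB_Dialogue widget that shows the NPC's portrait.
; Finishing marks the dialogue viewed, which reveals the skip text and lets SkipDialogue close it early on replays.
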(event OnComponentBeginOverlap(Collider)
  (params (OverlappedComponent :type Primitive%20Component%20Object%20Reference) (OtherActor :type Actor%20Object%20Reference) (OtherComp :type Primitive%20Component%20Object%20Reference) (OtherBodyIndex :type Integer) (bFromSweep :type Boolean) (SweepResult :type Hit%20Result%20Structure%20%28by%20ref%29))
  ;[1 1 1] When player leaves collider dialogue disappears and resets - CF
  (bind _asbp_third_person_character (Utilities|Casting|CastToBP_ThirdPersonCharacter OtherActor))
  (Widget|SetVisibility (Variables|/Game/Dynamic/ThirdPerson/Blueprints/WB_PlayerHUD.WB_PlayerHUD_C|GetInteract_Container (Variables|/Game/Dynamic/ThirdPerson/Blueprints/BP_ThirdPersonCharacter.BP_ThirdPersonCharacter_C|GetPlayerHUD _asbp_third_person_character)) "Visible"))

(event OnComponentEndOverlap(Collider)
  (params (OverlappedComponent :type Primitive%20Component%20Object%20Reference) (OtherActor :type Actor%20Object%20Reference) (OtherComp :type Primitive%20Component%20Object%20Reference) (OtherBodyIndex :type Integer))
  ;[1 1 1] When player leaves collider dialogue disappears and resets - CF
  (bind _asbp_third_person_character (Utilities|Casting|CastToBP_ThirdPersonCharacter OtherActor))
  (Widget|SetVisibility (Variables|/Game/Dynamic/ThirdPerson/Blueprints/WB_PlayerHUD.WB_PlayerHUD_C|GetInteract_Container (Variables|/Game/Dynamic/ThirdPerson/Blueprints/BP_ThirdPersonCharacter.BP_ThirdPersonCharacter_C|GetPlayerHUD _asbp_third_person_character)) "Hidden")
  (Variables|Default|SetTalkIndex -1)
  (if (Utilities|IsValid (Variables|Default|GetWidget))
    (Widget|SetVisibility (Variables|Default|GetWidget) "Hidden")))

(event EventBeginPlay
  (Sprite|SetFlipbook (Variables|Default|GetCharacterMesh) (Variables|Default|GetCharacterFlipBook)))

(event EventTalk
  ;[1 1 1] NPC Talk - CF
  (if (Variables|Default|GetSkipActive?)
    (Widget|SetVisibility (Variables|Default|GetWidget) "Hidden" :!label _label)
    (Variables|Default|SetTalkIndex -1)
    (Variables|Default|SetPreviouslyViewed? true)
    (Variables|Default|SetSkipActive? false)
    (else
      (Math|Integer|IncrementInt (Variables|Default|GetTalkIndex)
        (:%20%20
          (if (< (Variables|Default|GetTalkIndex) (Utilities|Array|Length (Variables|Default|GetDialogue)))
            (if (Variables|Default|GetPreviouslyViewed?)
              (Variables|/Script/UMG.Widget|SetVisibility (Variables|/Game/Dynamic/Blueprints/NPC/WB_Dialogue.WB_Dialogue_C|GetSkipText (Variables|Default|GetWidget)) "Visible"))
            (bind _widget (Variables|Default|GetWidget)
              (:then
                (Widget|SetVisibility _widget "Visible"))
              (:else
                (bind _returnvalue (UserInterface|CreateWidget "/Game/Dynamic/Blueprints/NPC/WB_Dialogue.WB_Dialogue_C" (Game|GetPlayerController 0)))
                (bind _output_get (Variables|Default|SetWidget _returnvalue))
                (UserInterface|Viewport|AddtoViewport _output_get 0)
                (Default|UpdatePortrait (Variables|Default|GetWidget) self)))
            (Rendering|Components|TextRender|SetText (Variables|/Game/Dynamic/Blueprints/NPC/WB_Dialogue.WB_Dialogue_C|GetTalkText (Variables|Default|GetWidget)) (Utilities|Text|ToText(String) (Utilities|Array|Get(acopy) (Variables|Default|GetDialogue) (Variables|Default|GetTalkIndex))))
            (else
              (goto _label))))))))

(event EventSkipDialogue
  ;[1 1 1] Skip Dialogue - CF
  (if (Variables|Default|GetPreviouslyViewed?)
    (Variables|Default|SetSkipActive? true)
    (CallFunction|Talk)))

(fn ConstructionScript)