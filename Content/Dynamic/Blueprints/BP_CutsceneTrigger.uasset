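; BP_CutsceneTrigger is a trigger volume that starts the final cutscene when the player character overlaps its collider.
; It creates the cutscene HUD widget at BeginPlay and adds it to the viewport on overlap.
; The overlap also sets the character's cutscene mode, disables input, destroys a crow enemy and flags the Level 3 music to stop.
; It then opens the cutscene media source and plays the "Lily of the Valley" track as 2D sound.
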(event OnComponentBeginOverlap(Collider)
  (params (OverlappedComponent :type Primitive%20Component%20Object%20Reference) (OtherActor :type Actor%20Object%20Reference) (OtherComp :type Primitive%20Component%20Object%20Reference) (OtherBodyIndex :type Integer) (bFromSweep :type Boolean) (SweepResult :type Hit%20Result%20Structure%20%28by%20ref%29))
  (bind _asbp_third_person_character (Utilities|Casting|CastToBP_ThirdPersonCharacter OtherActor))
  (Variables|/Game/Dynamic/ThirdPerson/Blueprints/BP_ThirdPersonCharacter.BP_ThirdPersonCharacter_C|SetCutsceneMode _asbp_third_person_character true)
  ;[1 1 1] Dev
  (Input|DisableInput _asbp_third_person_character (Game|GetPlayerController 0))
  (bind _returnvalue (Actor|GetActorOfClass "/Game/Dynamic/Blueprints/NPC/BP_Enemy_Crow.BP_Enemy_Crow_C"))
  (Utilities|IsValid _returnvalue
    (:Is%20Valid
      (Actor|DestroyActor _returnvalue))
    (:Is%20Not%20Valid
      _))
  (bind _returnvalue_2 (Actor|GetActorOfClass "/Game/Audio/Music/BP_Level3Music.BP_Level3Music_C"))
  (Variables|/Game/Audio/Music/BP_Level3Music.BP_Level3Music_C|SetStopIndefinitely _returnvalue_2 true)
  (UserInterface|Viewport|AddtoViewport (Variables|Default|GetHUD) 0)
  (Media|MediaPlayer|OpenSource (Variables|Default|GetMediaPlayer) "/Game/Movies/Final_cutscene.Final_cutscene")
  (Audio|PlaySound2D "/Game/Audio/Music/04_-_Lily_of_the_Valley.04_-_Lily_of_the_Valley" 1.0 1.0 0.0 0 0))

(event EventBeginPlay
  (bind _returnvalue (UserInterface|CreateWidget "/Game/Movies/FinalCutscene/WB_CutsceneHUD.WB_CutsceneHUD_C" (Game|GetPlayerController 0)))
  (Variables|Default|SetHUD _returnvalue))

(fn ConstructionScript)