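; Obstacle actor that damages the third-person character on contact, using a Paper2D flipbook as its visual and hit area.
; BeginPlay assigns the flipbook, disables looping and sets its starting frame.
; A Box overlap with the character plays the flipbook animation.
; A flipbook overlap subtracts one Health, destroys the character at zero or below, then destroys the obstacle itself.
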(event OnComponentBeginOverlap(Box)
  (params (OverlappedComponent :type Primitive%20Component%20Object%20Reference) (OtherActor :type Actor%20Object%20Reference) (OtherComp :type Primitive%20Component%20Object%20Reference) (OtherBodyIndex :type Integer) (bFromSweep :type Boolean) (SweepResult :type Hit%20Result%20Structure%20%28by%20ref%29))
  (Utilities|Casting|CastToBP_ThirdPersonCharacter OtherActor)
  (Audio|Components|Audio|Play (Variables|Default|GetObstacleFlipBook)))

(event OnComponentBeginOverlap(ObstacleFlipBook)
  (params (OverlappedComponent :type Primitive%20Component%20Object%20Reference) (OtherActor :type Actor%20Object%20Reference) (OtherComp :type Primitive%20Component%20Object%20Reference) (OtherBodyIndex :type Integer) (bFromSweep :type Boolean) (SweepResult :type Hit%20Result%20Structure%20%28by%20ref%29))
  ;[1 1 1] Deal 1 Damage - CF
  (bind _asbp_third_person_character (Utilities|Casting|CastToBP_ThirdPersonCharacter OtherActor))
  (bind _result (Math|Integer|DecrementInt (Variables|/Game/Dynamic/ThirdPerson/Blueprints/BP_ThirdPersonCharacter.BP_ThirdPersonCharacter_C|GetHealth _asbp_third_person_character))
    (:%20%20
      (Variables|/Game/Dynamic/ThirdPerson/Blueprints/BP_ThirdPersonCharacter.BP_ThirdPersonCharacter_C|SetHealth _asbp_third_person_character _result)
      (if (<= (Variables|/Game/Dynamic/ThirdPerson/Blueprints/BP_ThirdPersonCharacter.BP_ThirdPersonCharacter_C|GetHealth _asbp_third_person_character) 0)
        (Actor|DestroyActor _asbp_third_person_character))
      (Actor|DestroyActor))))

(event EventBeginPlay
  (Sprite|SetFlipbook (Variables|Default|GetObstacleFlipBook) (Variables|Default|GetFlipbook))
  (Components|Timeline|SetLooping (Variables|Default|GetObstacleFlipBook) false)
  (Class|PaperFlipbookComponent|SetPlaybackPositioninFrames (Variables|Default|GetObstacleFlipBook) 2 false))

(fn ConstructionScript)