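; BP_FlyingCameraTrigger is a trigger actor that changes the player's camera state, apparently for a flying camera mode, and shows enter or exit prompts.
; When BP_ThirdPersonCharacter begins overlapping the Collider, it calls UpdateCameraState on that character.
; A separate UpdatePrompt event, not called within this graph, uses a FlipFlop to alternate visibility of the Enter and Exit components, showing Exit first.
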(event OnComponentBeginOverlap(Collider)
  (params (OverlappedComponent :type Primitive%20Component%20Object%20Reference) (OtherActor :type Actor%20Object%20Reference) (OtherComp :type Primitive%20Component%20Object%20Reference) (OtherBodyIndex :type Integer) (bFromSweep :type Boolean) (SweepResult :type Hit%20Result%20Structure%20%28by%20ref%29))
  ;[1 1 1] Changes camera state when player collides with actor
  (bind _asbp_third_person_character (Utilities|Casting|CastToBP_ThirdPersonCharacter OtherActor))
  (Default|UpdateCameraState _asbp_third_person_character))

(event Custom|UpdatePrompt
  ;[1 1 1] Updates text when called
  (Utilities|FlowControl|FlipFlop
    (:A
      (Rendering|SetVisibility (Variables|Default|GetExit) true false)
      (Rendering|SetVisibility (Variables|Default|GetEnter) false false))
    (:B
      (Rendering|SetVisibility (Variables|Default|GetEnter) true false)
      (Rendering|SetVisibility (Variables|Default|GetExit) false false))))

(fn ConstructionScript)