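; BP_HouseSprite is an actor that shows a house as a sprite that always turns toward the player.
; On BeginPlay it applies its HouseSprite variable to the House sprite component.
; Each Tick it billboards on yaw only, using atan2 of the direction to BP_ThirdPersonCharacter plus a 90-degree offset, so it follows the character's position rather than the camera.
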(event EventTick
  (params (DeltaSeconds :type Float%20%28single-precision%29))
  ;[1 1 1] Rotates sprite to always face player - CF
  (bind _asbp_third_person_character (Utilities|Casting|CastToBP_ThirdPersonCharacter (Game|GetPlayerCharacter 0)))
  (Transformation|SetActorRotation (Math|Rotator|MakeRotator 0.0 0.0 (+ (Class|KismetMathLibrary|DegAtan2 (.y (- (Transformation|GetActorLocation _asbp_third_person_character) (Transformation|GetActorLocation))) (.x (- (Transformation|GetActorLocation _asbp_third_person_character) (Transformation|GetActorLocation)))) 9e+01))))

(event EventBeginPlay
  ;[1 1 1] Sets sprite
  (Rendering|Components|Sprite|SetSprite (Variables|Default|GetHouse) (Variables|Default|GetHouseSprite)))

(fn ConstructionScript)