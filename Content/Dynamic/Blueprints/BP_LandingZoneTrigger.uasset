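; BP_LandingZoneTrigger is a landing zone that lets the player start or stop flying with the interact input.
; Collider overlap toggles input and the HUD interact prompt for BP_ThirdPersonCharacter.
; Interact passes LZType to the character's flying and camera updates; one type also rejoins the spline, disables input and clears the cooldown after a delay.
; On BeginPlay, that same type sets a "Press to fly" prompt and shows the exit marker instead of the enter one.
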(event OnComponentBeginOverlap(Collider)
  (params (OverlappedComponent :type Primitive%20Component%20Object%20Reference) (OtherActor :type Actor%20Object%20Reference) (OtherComp :type Primitive%20Component%20Object%20Reference) (OtherBodyIndex :type Integer) (bFromSweep :type Boolean) (SweepResult :type Hit%20Result%20Structure%20%28by%20ref%29))
  ;[1 1 1] allow player input - CF
  (bind _asbp_third_person_character (Utilities|Casting|CastToBP_ThirdPersonCharacter OtherActor))
  (Input|EnableInput (Game|GetPlayerController 0))
  (Rendering|Components|TextRender|SetText (Variables|/Game/Dynamic/ThirdPerson/Blueprints/WB_PlayerHUD.WB_PlayerHUD_C|GetInteract_Description (Variables|/Game/Dynamic/ThirdPerson/Blueprints/BP_ThirdPersonCharacter.BP_ThirdPersonCharacter_C|GetPlayerHUD _asbp_third_person_character)) (Variables|Default|GetPromptText))
  (Widget|SetVisibility (Variables|/Game/Dynamic/ThirdPerson/Blueprints/WB_PlayerHUD.WB_PlayerHUD_C|GetInteract_Container (Variables|/Game/Dynamic/ThirdPerson/Blueprints/BP_ThirdPersonCharacter.BP_ThirdPersonCharacter_C|GetPlayerHUD _asbp_third_person_character)) "Visible"))

(event OnComponentEndOverlap(Collider)
  (params (OverlappedComponent :type Primitive%20Component%20Object%20Reference) (OtherActor :type Actor%20Object%20Reference) (OtherComp :type Primitive%20Component%20Object%20Reference) (OtherBodyIndex :type Integer))
  ;[1 1 1] allow player input - CF
  (bind _asbp_third_person_character (Utilities|Casting|CastToBP_ThirdPersonCharacter OtherActor))
  (Input|DisableInput (Game|GetPlayerController 0))
  (Default|ResetInteract (Variables|/Game/Dynamic/ThirdPerson/Blueprints/BP_ThirdPersonCharacter.BP_ThirdPersonCharacter_C|GetPlayerHUD _asbp_third_person_character))
  (Widget|SetVisibility (Variables|/Game/Dynamic/ThirdPerson/Blueprints/WB_PlayerHUD.WB_PlayerHUD_C|GetInteract_Container (Variables|/Game/Dynamic/ThirdPerson/Blueprints/BP_ThirdPersonCharacter.BP_ThirdPersonCharacter_C|GetPlayerHUD _asbp_third_person_character)) "Hidden"))

(event Input|EnhancedActionEvents|EnhancedInputActionIA_Interact
  (params (ActionValue :type Boolean) (ElapsedSeconds :type Float%20%28double-precision%29) (TriggeredSeconds :type Float%20%28double-precision%29) (InputAction :type Input%20Action%20Object%20Reference :default "/Game/Dynamic/ThirdPerson/Input/Actions/IA_Interact.IA_Interact"))
  (bind _lztype (Variables|Default|GetLZType))
  ;[1 1 1] Stop/Start Flying - CF
  (:Triggered
    (if (not (Variables|Default|GetCooldownActive))
      (Variables|Default|SetCooldownActive true)
      (bind _asbp_third_person_character (Utilities|Casting|CastToBP_ThirdPersonCharacter (Game|GetPlayerCharacter 0)))
      (Default|TriggerFlying _asbp_third_person_character _lztype)
      (Default|UpdateCameraState _asbp_third_person_character _lztype)
      (if (Utilities|Enum|Equal(Enum) "NewEnumerator0" _lztype)
        (Default|RejoinSpline (Variables|/Game/Dynamic/ThirdPerson/Blueprints/BP_ThirdPersonCharacter.BP_ThirdPersonCharacter_C|GetCurrentSpline _asbp_third_person_character))
        (Default|RejoinSpline _asbp_third_person_character)
        (Input|DisableInput (Game|GetPlayerController 0))
        (Utilities|FlowControl|Delay 1.0)
        (Variables|Default|SetCooldownActive false)))))

(event EventBeginPlay
  ;[1 1 1] Update Prompt On LZ Type - CF
  (if (Utilities|Enum|Equal(Enum) (Variables|Default|GetLZType) "NewEnumerator0")
    (Variables|Default|SetPromptText "Press to fly")
    (Rendering|SetVisibility (Variables|Default|GetLandingZoneExit) true false)
    (Rendering|SetVisibility (Variables|Default|GetLandingZoneEnter) false false)))

(fn ConstructionScript)