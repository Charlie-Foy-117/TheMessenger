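; BP_Package is a pickup actor that the player collects with the interact input.
; Its collider overlap with the third-person character toggles the actor's input and a visible prompt.
; On interact it adds itself to the character's inventory component, updates the quest, then hides itself and disables collision instead of being destroyed.
; It also notifies every Bp_LockedDoor in the level that a package was picked up.
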(event OnComponentBeginOverlap(Collider)
  (params (OverlappedComponent :type Primitive%20Component%20Object%20Reference) (OtherActor :type Actor%20Object%20Reference) (OtherComp :type Primitive%20Component%20Object%20Reference) (OtherBodyIndex :type Integer) (bFromSweep :type Boolean) (SweepResult :type Hit%20Result%20Structure%20%28by%20ref%29))
  ;[1 1 1] Input Access - CF
  (Utilities|Casting|CastToBP_ThirdPersonCharacter OtherActor)
  (Input|EnableInput (Game|GetPlayerController 0))
  (Rendering|SetVisibility (Variables|Default|GetPrompt) true false))

(event OnComponentEndOverlap(Collider)
  (params (OverlappedComponent :type Primitive%20Component%20Object%20Reference) (OtherActor :type Actor%20Object%20Reference) (OtherComp :type Primitive%20Component%20Object%20Reference) (OtherBodyIndex :type Integer))
  ;[1 1 1] Input Access - CF
  (Utilities|Casting|CastToBP_ThirdPersonCharacter OtherActor)
  (Input|DisableInput (Game|GetPlayerController 0))
  (Rendering|SetVisibility (Variables|Default|GetPrompt) false false))

(event Input|EnhancedActionEvents|EnhancedInputActionIA_Interact
  (params (ActionValue :type Boolean) (ElapsedSeconds :type Float%20%28double-precision%29) (TriggeredSeconds :type Float%20%28double-precision%29) (InputAction :type Input%20Action%20Object%20Reference :default "/Game/Dynamic/ThirdPerson/Input/Actions/IA_Interact.IA_Interact"))
  ;[1 1 1] Pick up package - CF
  (:Triggered
    (bind _asbp_third_person_character (Utilities|Casting|CastToBP_ThirdPersonCharacter (Game|GetPlayerCharacter 0)))
    (Default|AddItemtoPackages (Variables|/Game/Dynamic/ThirdPerson/Blueprints/BP_ThirdPersonCharacter.BP_ThirdPersonCharacter_C|GetBPC_Inventory _asbp_third_person_character) self)
    (Default|UpdateQuest _asbp_third_person_character)
    (Rendering|SetActorHiddenInGame true)
    (Collision|SetCollisionEnabled (Variables|Default|GetCollider) "NoCollision")
    ;[1 1 1] Check is Bp_lockeddoor should be destroyed - CF
    (bind _outactors (Actor|GetAllActorsOfClass "/Game/Dynamic/Blueprints/Bp_LockedDoor.Bp_LockedDoor_C"))
    (Default|PickedUpPackage _outactors)))

(fn ConstructionScript)